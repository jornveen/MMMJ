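; Player Blueprint that turns switch inputs (left, right, or players 1 to 4) into action requests for the game mode.
; BeginPlay caches GameMode_MMMJ, and each input press passes an action enum to SetAction.
; SetAction forwards it with this PlayerID to the game mode unless the enum's integer value equals that ID.
; Unconnected direct switch calls to the game mode remain in the graph.
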(event `self.ReceiveBeginPlay`
  (bind _asgame_mode_mmmj (cast `/Game/Blueprints/GameMode_MMMJ` (`GameplayStatics.GetGameMode`))
    (:`then`
      (set `self.GameMode` _asgame_mode_mmmj))
    (:`CastFailed`
      (`KismetSystemLibrary.PrintString` "Gamemode not found"))))

(event `InputAction|SwitchRight`
  (params (Key :type "Key Structure"))
  (:`Pressed`
    (`self.SetAction` "NewEnumerator1")))

(event `InputAction|SwitchLeft`
  (params (Key :type "Key Structure"))
  (:`Pressed`
    (`self.SetAction` "NewEnumerator0")))

(event `InputAction|SwitchPlayer1`
  (params (Key :type "Key Structure"))
  (:`Pressed`
    (`self.SetAction` "NewEnumerator2")))

(event `InputAction|SwitchPlayer2`
  (params (Key :type "Key Structure"))
  (:`Pressed`
    (`self.SetAction` "NewEnumerator3")))

(event `InputAction|SwitchPlayer3`
  (params (Key :type "Key Structure"))
  (:`Pressed`
    (`self.SetAction` "NewEnumerator4")))

(event `InputAction|SwitchPlayer4`
  (params (Key :type "Key Structure"))
  (:`Pressed`
    (`self.SetAction` "NewEnumerator5")))

(event `InputAction|SwitchRight`
  (params (Key :type "Key Structure")))

(event `InputAction|SwitchLeft`
  (params (Key :type "Key Structure")))

(event `InputAction|SwitchPlayer2`
  (params (Key :type "Key Structure")))

(event `InputAction|SwitchPlayer3`
  (params (Key :type "Key Structure")))

(event `InputAction|SwitchPlayer4`
  (params (Key :type "Key Structure")))

(fn `SetAction`
  (params (Action :type "/Game/Enums/ActionTypes Enum" :default "NewEnumerator2"))
  (if (not (== (`KismetMathLibrary.Conv_ByteToInt` Action) (`self.PlayerID`)))
    (`/Game/Blueprints/GameMode_MMMJ.SetAction` (`self.GameMode`) (`self.PlayerID`) Action)))

(fn `UserConstructionScript`)