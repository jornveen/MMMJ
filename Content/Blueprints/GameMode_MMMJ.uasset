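; Game mode for a local four-player bomb-passing party game, where players shuffle boxes to avoid holding the Box_Boom.
; Tick alternates a timed choice phase with spaced execution of swap or shift actions, in a player order that rotates each turn.
; After KillTurnCount turns the bomb holder loses HP, possibly dying, and the bomb moves randomly.
; With two players left, a timed duel lets the holder pass the bomb on a cooldown.
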(event `self.ReceiveBeginPlay`
  (set `self.RoundTimer` (`self.RoundTime`))
  (set `self.ActionTimer` (`self.ActionTime`))
  (set `self.SwitchTimer` (`self.SwitchTime`))
  (set `self.BattleTimer` (`self.BattleTime`))
  (`self.Set/GetBoxes`)
  (`self.SetupPlayers`)
  (`self.GiveRandomPlayerBoom`)
  (bind _returnvalue (`|CreateWidget` "/Game/Blueprints/W_Testlayout.W_Testlayout_C"))
  (bind _output_get (set `self.W_ChoiceMenu` _returnvalue))
  (`UserWidget.AddToViewport` _output_get 0))

(event `self.ReceiveTick`
  (params (DeltaSeconds :type "Float (single-precision)"))
  (bind _actionindex (`self.ActionIndex`))
  (bind _returnvalue (+ _actionindex 1))
  (if (`self.GameEnded`)
    _
    (elif (`self.OneVSOneBattleActive`)
      (`self.OneVSOneBattle` DeltaSeconds)
      (elif (== (`self.TurnCounter`) (`self.KillTurnCount`))
        (`self.KillPlayer`)
        (set `self.TurnCounter` 0)
        (`self.GiveRandomPlayerBoom`)
        (bind _playeralive (`self.GetNumerOfPlayersAlive`))
        (if (== _playeralive 2)
          (set `self.OneVSOneBattleActive` true)
          (set `self.CanSetActions` false))
        (elif (`self.CanSetActions`)
          (`self.UpdateRoundTimer` DeltaSeconds)
          (if (<= (`self.RoundTimer`) 0.0)
            (set `self.CanSetActions` false)
            (`KismetSystemLibrary.Delay` 1.0)
            (`Widget.SetVisibility` (`self.W_ChoiceMenu`) "Hidden"))
          (elif (`self.CanExecuteAction`)
            (set `self.CanExecuteAction` false)
            (`self.ExecuteActions` (`|GetArrayItem` (`self.ActionIndexer`) _actionindex))
            (`self.SetHasBoom`)
            (if (== _returnvalue 4)
              (set `self.ActionIndex` 0)
              (set `self.CanSetActions` true)
              (set `self.RoundTimer` (`self.RoundTime`))
              (`/Engine/EditorBlueprintResources/StandardMacros.IncrementInt` (`self.TurnCounter`)
                (:`  `
                  (`Widget.SetVisibility` (`self.W_ChoiceMenu`) "Visible")
                  (`self.ResetUIInput`)
                  (`self.UpdateActionIndexer`)))
              (else
                (set `self.ActionIndex` _returnvalue)))
            (else
              (bind _output_get (set `self.ActionTimer` (- (`self.ActionTimer`) DeltaSeconds)))
              (if (<= _output_get 0.0)
                (set `self.CanExecuteAction` true)
                (set `self.ActionTimer` (`self.ActionTime`))))))))))

(fn `ExecuteActions`
  (params (ActionIndex :type Integer))
  (if (`|GetArrayItem` (`self.IsPlayerDead`) ActionIndex)
    (set `self.ActionTimer` 0.0)
    (else
      (switch `/Game/Enums/ActionTypes` (`|GetArrayItem` (`self.Actions`) ActionIndex)
        (:`NewEnumerator2`
          (`self.SwitchPlayer` ActionIndex))
        (:`NewEnumerator3`
          (`self.SwitchPlayer` ActionIndex 1))
        (:`NewEnumerator4`
          (`self.SwitchPlayer` ActionIndex 2))
        (:`NewEnumerator5`
          (`self.SwitchPlayer` ActionIndex 3))
        (:`NewEnumerator1`
          (`self.SwitchRight`))
        (:`NewEnumerator0`
          (`self.SwitchLeft`))))))

(fn `GetBox`
  (params (PlayerID :type Integer))
  (returns (Box_Normal :type "/Game/Blueprints/Box_Normal Object Reference"))
  (for _array_element (`self.Boxes`)
    (if (== (`/Game/Blueprints/Box_Normal.OwnerID` _array_element) PlayerID)
      (return _array_element))))

(fn `GetNumerOfPlayersAlive`
  (returns (PlayerAlive :type Integer))
  (locals (NumberOfPlayers :type Integer))
  (set `local.NumberOfPlayers` (`KismetArrayLibrary.Array_Length` (`self.IsPlayerDead`)))
  (for _array_element (`self.IsPlayerDead`)
    (if _array_element
      (`/Engine/EditorBlueprintResources/StandardMacros.DecrementInt` (`local.NumberOfPlayers`))))
  (return (`local.NumberOfPlayers`)))

(fn `GiveRandomPlayerBoom`
  (locals (RandomInt :type Integer) (Box :type "/Game/Blueprints/Box_Normal Object Reference") (Temp_OwnerID :type Integer))
  (bind _output (`|GetArrayItem` (`self.Boxes`) (`local.RandomInt`)))
  (bind _output_2 (`|GetArrayItem` (`self.Boxes`) (`local.RandomInt`)))
  (bind _outactors (`GameplayStatics.GetAllActorsOfClass` "/Game/Blueprints/Box_Boom.Box_Boom_C"))
  (set `local.RandomInt` (`KismetMathLibrary.RandomInteger` (`KismetArrayLibrary.Array_LastIndex` (`self.Boxes`))))
  (set `local.Box` _output_2)
  (set `local.Temp_OwnerID` (`/Game/Blueprints/Box_Normal.OwnerID` _output_2))
  (bind _output_3 (`|GetArrayItem` _outactors))
  (if (`|GetArrayItem` (`self.IsPlayerDead`) (`/Game/Blueprints/Box_Normal.OwnerID` _output_3))
    (`SceneComponent.SetVisibility` (`/Game/Blueprints/Box_Normal.Box` (`|GetArrayItem` (`self.Boxes`) (`local.RandomInt`))) false false)
    (`KismetArrayLibrary.Array_Set` (`self.Boxes`) (`local.RandomInt`) _output_3 :!label _label)
    (bind _output_get (set `/Game/Blueprints/Box_Normal.OwnerID` (`local.Temp_OwnerID`) _output_3))
    (`self.SetBoxLocation` _output_get _output_3)
    (`self.SetHasBoom`)
    (else
      (for (_array_element _array_index) (`self.Boxes`)
        (bind _asbox_boom (cast `/Game/Blueprints/Box_Boom` _array_element))
        (`KismetArrayLibrary.Array_Set` (`self.Boxes`) _array_index _output)
        (bind _output_get_2 (set `/Game/Blueprints/Box_Normal.OwnerID` (`/Game/Blueprints/Box_Normal.OwnerID` _asbox_boom) _output))
        (`self.SetBoxLocation` _output_get_2 _output)
        (goto _label)))))

(fn `KillPlayer`
  (for (_array_element _array_index) (`self.HasBoom`)
    (if _array_element
      (if (not (`|GetArrayItem` (`self.IsPlayerDead`) _array_index))
        (bind _output (`|GetArrayItem` (`self.Players`) _array_index))
        (bind _output_get (set `/Game/Blueprints/Player.PlayerHp` (- (`/Game/Blueprints/Player.PlayerHp` _output) 1) _output))
        (if (<= _output_get 0)
          (`KismetArrayLibrary.Array_Set` (`self.IsPlayerDead`) _array_index true)
          (`KismetArrayLibrary.Array_Remove` (`self.Boxes`) _array_index))))))

(fn `OneVSOneBattle`
  (params (DeltaTime :type "Float (double-precision)"))
  (`self.UpdateBattleTimer` DeltaTime)
  (if (<= (`self.BattleTimer`) 0.0)
    (`self.KillPlayer`)
    (set `self.GameEnded` true)
    (elif (not (`self.CanSwitch`))
      (`self.UpdateSwitchTimer` DeltaTime)
      (if (<= (`self.SwitchTimer`) 0.0)
        (set `self.CanSwitch` true)
        (set `self.SwitchTimer` (`self.SwitchTime`))))))

(fn `ResetUIInput`
  (for _array_element (`self.Players`)
    (bind _playerid (`/Game/Blueprints/Player.PlayerID` _array_element))
    (`KismetArrayLibrary.Array_Set` (`self.Actions`) _playerid "NewEnumerator0")
    (`/Game/Blueprints/W_Testlayout.PlayerInput` (`self.W_ChoiceMenu`) _playerid 4)))

(fn `Set/GetBoxes`
  (bind _outactors (`GameplayStatics.GetAllActorsOfClass` "/Game/Blueprints/Box_Normal.Box_Normal_C"))
  (bind _output_get (set `self.Boxes` _outactors))
  (for (_array_element _array_index) _output_get
    (set `/Game/Blueprints/Box_Normal.OwnerID` _array_index _array_element)
    (`self.K2_SetActorLocation` _array_element (`|GetArrayItem` (`self.ObjectPositions`) _array_index) false true)
    (cast `/Game/Blueprints/Box_Boom` _array_element)
    (`KismetArrayLibrary.Array_Set` (`self.HasBoom`) _array_index true)))

(fn `SetAction`
  (params (PlayerID :type Integer) (Action :type "/Game/Enums/ActionTypes Enum" :default "NewEnumerator2"))
  (returns (CanExecute :type Boolean))
  (if (`self.CanSetActions`)
    (if (`|GetArrayItem` (`self.IsPlayerDead`) PlayerID)
      _
      (else
        (`KismetArrayLibrary.Array_Set` (`self.Actions`) PlayerID Action)
        (return true))))
  (return false))

(fn `SetBoxLocation`
  (params (IndexLocation :type Integer) (Box :type "/Game/Blueprints/Box_Normal Object Reference"))
  (`self.K2_SetActorLocation` Box (`|GetArrayItem` (`self.ObjectPositions`) IndexLocation) false true))

(fn `SetHasBoom`
  (set `self.HasBoom` (`|MakeArray` false false false false))
  (for _array_element (`self.Boxes`)
    (cast `/Game/Blueprints/Box_Boom` _array_element)
    (`KismetArrayLibrary.Array_Set` (`self.HasBoom`) (`/Game/Blueprints/Box_Normal.OwnerID` _array_element) true)))

(fn `SetupPlayers`
  (for _ (range 3)
    (`GameplayStatics.CreatePlayer` -1))
  (bind _outactors (`GameplayStatics.GetAllActorsOfClass` "/Game/Blueprints/Player.Player_C"))
  (for (_array_element _array_index) _outactors
    (set `/Game/Blueprints/Player.PlayerID` _array_index _array_element)
    (`Controller.Possess` (`GameplayStatics.GetPlayerController` _array_index) _array_element)
    (`KismetArrayLibrary.Array_Add` (`self.Players`) _array_element)))

(fn `SwitchBoom`
  (params (PlayerID :type Integer))
  (if (`self.CanSwitch`)
    (if (`|GetArrayItem` (`self.HasBoom`) PlayerID)
      (`self.SwitchLeft`)
      (`self.SetHasBoom`)
      (set `self.CanSwitch` false))))

(fn `SwitchLeft`
  (locals (Temp_Boxes :type "Array of /Game/Blueprints/Box_Normal Object Reference") (Temp_Owners :type "Array of Integer"))
  (bind _boxes (`self.Boxes`))
  (bind _returnvalue (`KismetArrayLibrary.Array_LastIndex` _boxes))
  (bind _output (`|GetArrayItem` (`local.Temp_Owners`) _returnvalue))
  (`KismetArrayLibrary.Array_Clear` (`local.Temp_Owners`))
  (`KismetArrayLibrary.Array_Clear` (`local.Temp_Boxes`))
  (for _array_element (`self.Boxes`)
    (`KismetArrayLibrary.Array_Add` (`local.Temp_Boxes`) _array_element)
    (`KismetArrayLibrary.Array_Add` (`local.Temp_Owners`) (`/Game/Blueprints/Box_Normal.OwnerID` _array_element)))
  (for (_array_element_2 _array_index) (`local.Temp_Boxes`)
    (if (== _array_index 0)
      (`KismetArrayLibrary.Array_Set` _boxes _returnvalue _array_element_2)
      (`self.SetBoxLocation` _output _array_element_2)
      (set `/Game/Blueprints/Box_Normal.OwnerID` _output _array_element_2)
      (else
        (bind _returnvalue_2 (+ _array_index -1))
        (`KismetArrayLibrary.Array_Set` (`self.Boxes`) _returnvalue_2 _array_element_2)
        (bind _output_2 (`|GetArrayItem` (`local.Temp_Owners`) _returnvalue_2))
        (`self.SetBoxLocation` _output_2 _array_element_2)
        (set `/Game/Blueprints/Box_Normal.OwnerID` _output_2 _array_element_2)))))

(fn `SwitchPlayer`
  (params (PlayerID :type Integer) (PlayerSwitchID :type Integer))
  (locals (Box1 :type "/Game/Blueprints/Box_Normal Object Reference") (Box2 :type "/Game/Blueprints/Box_Normal Object Reference") (Temp_Owner1 :type Integer) (Temp_Owner2 :type Integer))
  (set `local.Temp_Owner1` PlayerID)
  (set `local.Temp_Owner2` PlayerSwitchID)
  (bind _box_normal (`self.GetBox` (`local.Temp_Owner1`)))
  (set `local.Box1` _box_normal)
  (bind _box_normal_2 (`self.GetBox` (`local.Temp_Owner2`)))
  (set `local.Box2` _box_normal_2)
  (`KismetArrayLibrary.Array_Set` (`self.Boxes`) (`local.Temp_Owner1`) (`local.Box2`))
  (`self.SetBoxLocation` (`local.Temp_Owner1`) (`local.Box2`))
  (`KismetArrayLibrary.Array_Set` (`self.Boxes`) (`local.Temp_Owner2`) (`local.Box1`))
  (`self.SetBoxLocation` (`local.Temp_Owner2`) (`local.Box1`))
  (set `/Game/Blueprints/Box_Normal.OwnerID` (`local.Temp_Owner2`) (`local.Box1`))
  (set `/Game/Blueprints/Box_Normal.OwnerID` (`local.Temp_Owner1`) (`local.Box2`)))

(fn `SwitchRight`
  (locals (Temp_Boxes :type "Array of /Game/Blueprints/Box_Normal Object Reference") (Temp_Owners :type "Array of Integer"))
  (bind _output (`|GetArrayItem` (`self.Boxes`)))
  (bind _output_2 (`|GetArrayItem` (`local.Temp_Owners`)))
  (`KismetArrayLibrary.Array_Clear` (`local.Temp_Owners`))
  (`KismetArrayLibrary.Array_Clear` (`local.Temp_Boxes`))
  (for _array_element (`self.Boxes`)
    (`KismetArrayLibrary.Array_Add` (`local.Temp_Boxes`) _array_element)
    (`KismetArrayLibrary.Array_Add` (`local.Temp_Owners`) (`/Game/Blueprints/Box_Normal.OwnerID` _array_element)))
  (for (_array_element_2 _array_index) (`local.Temp_Boxes`)
    (if (== _array_index (`KismetArrayLibrary.Array_LastIndex` (`self.Boxes`)))
      (`KismetArrayLibrary.Array_Set` (`self.Boxes`) 0 _array_element_2)
      (`self.SetBoxLocation` _output_2 _output)
      (set `/Game/Blueprints/Box_Normal.OwnerID` _output_2 _output)
      (else
        (bind _returnvalue (+ _array_index 1))
        (`KismetArrayLibrary.Array_Set` (`self.Boxes`) _returnvalue _array_element_2)
        (bind _output_3 (`|GetArrayItem` (`local.Temp_Owners`) _returnvalue))
        (bind _output_4 (`|GetArrayItem` (`self.Boxes`) _returnvalue))
        (`self.SetBoxLocation` _output_3 _output_4)
        (set `/Game/Blueprints/Box_Normal.OwnerID` _output_3 _output_4)))))

(fn `UpdateActionIndexer`
  (bind _actionindexer (`self.ActionIndexer`))
  (bind _output (`|GetArrayItem` (`self.ActionIndexer`)))
  (for (_array_element _array_index) (`self.ActionIndexer`)
    (bind _returnvalue (+ _array_element 1))
    (if (== _returnvalue 4)
      (`KismetArrayLibrary.Array_Set` _actionindexer _array_index)
      (else
        (`KismetArrayLibrary.Array_Set` _actionindexer _array_index _returnvalue))))
  (if (`|GetArrayItem` (`self.IsPlayerDead`) _output)
    (`self.UpdateActionIndexer`)
    (else
      (`/Game/Blueprints/W_Testlayout.SetPlayerStart` (`self.W_ChoiceMenu`) _output))))

(fn `UpdateBattleTimer`
  (params (DeltaTime :type "Float (double-precision)"))
  (bind _output_get (set `self.BattleTimer` (- (`self.BattleTimer`) DeltaTime)))
  (`TextBlock.SetText` (`/Game/Blueprints/W_Testlayout.TimerText` (`self.W_ChoiceMenu`)) (`KismetTextLibrary.Conv_IntToText` (`KismetMathLibrary.Round` _output_get))))

(fn `UpdateRoundTimer`
  (params (DeltaTime :type "Float (double-precision)"))
  (bind _output_get (set `self.RoundTimer` (- (`self.RoundTimer`) DeltaTime)))
  (`TextBlock.SetText` (`/Game/Blueprints/W_Testlayout.TimerText` (`self.W_ChoiceMenu`)) (`KismetTextLibrary.Conv_IntToText` (`KismetMathLibrary.Round` _output_get))))

(fn `UpdateSwitchTimer`
  (params (DeltaTime :type "Float (double-precision)"))
  (set `self.SwitchTimer` (- (`self.SwitchTimer`) DeltaTime)))

(fn `UserConstructionScript`)